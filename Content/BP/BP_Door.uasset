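; Replicated interactable door that swings open and closed, usable while a first-person character overlaps its box trigger.
; Interaction calls a server event that flips IsOpen, whose OnRep runs OpenDoor with player character 0 on each machine.
; A timeline rotates the mesh or reverses to close, choosing swing direction by dotting the character's offset with the root's world location rather than a facing vector.
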(event `self.Box.OnComponentBeginOverlap`
  (params (OverlappedComponent :type "PrimitiveComponent Object Reference") (OtherActor :type "Actor Object Reference") (OtherComp :type "PrimitiveComponent Object Reference") (OtherBodyIndex :type Integer) (bFromSweep :type Boolean) (SweepResult :type "HitResult Structure (by ref)"))
  (cast `/Game/FirstPerson/Blueprints/BP_FirstPersonCharacter` OtherActor)
  (set `self.canInteract` true))

(event `self.Box.OnComponentEndOverlap`
  (params (OverlappedComponent :type "PrimitiveComponent Object Reference") (OtherActor :type "Actor Object Reference") (OtherComp :type "PrimitiveComponent Object Reference") (OtherBodyIndex :type Integer))
  (cast `/Game/FirstPerson/Blueprints/BP_FirstPersonCharacter` OtherActor)
  (set `self.canInteract` false))

(event `/Game/BP/I_Interact.OnInteract`
  (params (Character :type "Character Object Reference"))
  (`self.Server_OpenDoor` Character))

(event `Server_OpenDoor`
  (params (Character :type "Character Object Reference"))
  (set `self.isOpen` (not (`self.isOpen`))))

(event `Multicast_Open_Door`
  (params (Character :type "Character Object Reference")))

(event `Open Door`
  (params (cHA :type "Character Object Reference"))
  (bind _isopen (`self.isOpen`))
  (bind _returnvalue (`SceneComponent.K2_GetComponentLocation` (`self.DefaultSceneRoot`)))
  (`KismetSystemLibrary.PrintString` (`KismetStringLibrary.Conv_BoolToString` _isopen))
  (if _isopen
    (bind _output_get (set `self.endRotation` (`KismetMathLibrary.SelectFloat` 90.0 -90.0 (>= (`KismetMathLibrary.Dot_VectorVector` (`KismetMathLibrary.Normal` (- (`self.K2_GetActorLocation` cHA) _returnvalue)) _returnvalue) 0.0))))
    (bind (_direction _dooropen) (`Timeline|Timeline` :!label _label)
      (:`Update`
        (`SceneComponent.K2_SetRelativeRotation` (`self.StaticMesh`) (`KismetMathLibrary.MakeRotator` 0.0 90.0 (* _dooropen _output_get)) false false)))
    (else
      (goto _label :!via `Reverse`))))

(fn `IsInteractable`
  (returns (isInteractable :type Boolean))
  (return (`self.canInteract`)))

(fn `OnHit`
  (params (Damage :type "Float (double-precision)") (Object :type "/Game/current_FirstPerson/Blueprints/BP_FirstPersonProjectile Object Reference"))
  (return))

(fn `OnRep_isOpen`
  (`self.Open Door` (`GameplayStatics.GetPlayerCharacter` 0)))

(fn `UserConstructionScript`)