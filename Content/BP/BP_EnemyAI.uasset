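; Enemy AI character that hunts the first-person player, randomly set up as melee or ranged by its construction script.
; PawnSensing starts an AIMoveTo chase that leads to randomly delayed montage attacks: gunfire, or melee damage gated by a box overlap.
; A looping timer turns it toward the player during attacks.
; Being hit ragdolls it with a chance of score pickup, blood effect and sound; state-machine events are empty stubs.
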(event `SwitchState`
  (params (NewState :type Integer)))

(event `StateIdle`)

(event `StateFollow`)

(event `StateAttack`)

(event `self.ReceiveBeginPlay`)

(event `self.PawnSensing.OnSeePawn`
  (params (Pawn :type "Pawn Object Reference"))
  (set `self.CanSeePlayer?` true)
  (bind _asbp_first_person_character (cast `/Game/FirstPerson/Blueprints/BP_FirstPersonCharacter` Pawn))
  (set `self.Player` _asbp_first_person_character)
  (if (`self.Ranged?`)
    (`self.FollowPlayer_Ranged`)
    (else
      (`self.FollowPlayer_Melee`))))

(event `FollowPlayer_Ranged`
  (if (`self.CanSeePlayer?`)
    (set `self.isMoving` true)
    (`|AIMoveTo` self (0.0 0.0 0.0) (`self.Player`) 400.0
      (:`OnSuccess`
        (if (`self.CanAttack`)
          (`self.ShootPlayer`)
          (set `self.isMoving` false)
          (`self.FollowPlayer_Ranged`))))))

(event `FollowPlayer_Melee`
  (if (`self.CanSeePlayer?`)
    (set `self.isMoving` true)
    (`|AIMoveTo` self (0.0 0.0 0.0) (`self.Player`) 150.0
      (:`OnSuccess`
        (if (`self.CanAttack`)
          (`self.AttackPlayer`)
          (set `self.isMoving` false)
          (`self.FollowPlayer_Melee`))))))

(event `AttackPlayer`
  (`KismetSystemLibrary.K2_SetTimerDelegate` (delegate `RotateAI`) 0.01 true true)
  (set `self.CanAttack` false)
  (`KismetSystemLibrary.Delay` (+ (* (`KismetMathLibrary.RandomFloat`) 2.0) 0.5))
  (`self.PlayAnimMontage` "/Game/Sword_Animation/Animations/anim_attack_light_01_Montage.anim_attack_light_01_Montage" 1.0 (`KismetStringLibrary.Conv_StringToName` (`|GetArrayItem` (`self.LightAttacks`) (`KismetMathLibrary.RandomInteger` 2))))
  (if (`self.canHitPlayer`)
    (`/Game/FirstPerson/Blueprints/BP_FirstPersonCharacter.OnHitPlayer` (`self.Player`) 10.0 null))
  (set `self.CanAttack` true))

(event `ShootPlayer`
  (bind _wc_ranged (`self.WC_Ranged`))
  (if (not (`self.isDead`))
    (`KismetSystemLibrary.K2_SetTimerDelegate` (delegate `RotateAI`) 0.01 true true)
    (set `self.CanAttack` false)
    (`KismetSystemLibrary.Delay` (* (`KismetMathLibrary.RandomFloat`) 2.0))
    (`self.PlayAnimMontage` "/Game/AnimStarterPack/UE5_Upgraded/Fire_Rifle_Hip_Montage.Fire_Rifle_Hip_Montage" 1.0 "Default")
    (`KismetSystemLibrary.Delay` 0.3)
    (set `/Game/current_FirstPerson/Blueprints/BP_Weapon_Component_Enemy.FiringAt` (`self.Player`) _wc_ranged)
    (`/Game/current_FirstPerson/Blueprints/BP_Weapon_Component_Enemy.FireGun` _wc_ranged)
    (set `self.CanAttack` true)))

(event `RotateAI`
  (bind (_returnvalue_roll _returnvalue_pitch _returnvalue_yaw) (`KismetMathLibrary.BreakRotator` (`KismetMathLibrary.FindLookAtRotation` (`self.K2_GetActorLocation`) (`self.K2_GetActorLocation` (`self.Player`)))))
  (`self.K2_SetActorRotation` (`KismetMathLibrary.RInterpTo` (`self.K2_GetActorRotation`) (`KismetMathLibrary.MakeRotator` 0.0 0.0 _returnvalue_yaw) (`GameplayStatics.GetWorldDeltaSeconds`) 1.0)))

(event `CheckIfPlayerCanBeHit`
  (bind _returnvalue (`self.K2_GetActorRotation`))
  (bind _returnvalue_2 (`KismetMathLibrary.Vector_Normal2D` (- (`self.K2_GetActorLocation` (`GameplayStatics.GetPlayerController` 0)) (`self.K2_GetActorLocation`))))
  (`KismetSystemLibrary.PrintString` (`KismetStringLibrary.Conv_DoubleToString` (`KismetMathLibrary.DegAtan2` (`KismetMathLibrary.Dot_VectorVector` _returnvalue_2 (`KismetMathLibrary.Vector_Normal2D` (`KismetMathLibrary.GetRightVector` _returnvalue))) (`KismetMathLibrary.Dot_VectorVector` _returnvalue_2 (`KismetMathLibrary.Vector_Normal2D` (`KismetMathLibrary.GetForwardVector` _returnvalue)))))))

(event `self.Box.OnComponentBeginOverlap`
  (params (OverlappedComponent :type "PrimitiveComponent Object Reference") (OtherActor :type "Actor Object Reference") (OtherComp :type "PrimitiveComponent Object Reference") (OtherBodyIndex :type Integer) (bFromSweep :type Boolean) (SweepResult :type "HitResult Structure (by ref)"))
  (cast `/Game/FirstPerson/Blueprints/BP_FirstPersonCharacter` OtherActor)
  (set `self.canHitPlayer` true))

(event `self.Box.OnComponentEndOverlap`
  (params (OverlappedComponent :type "PrimitiveComponent Object Reference") (OtherActor :type "Actor Object Reference") (OtherComp :type "PrimitiveComponent Object Reference") (OtherBodyIndex :type Integer))
  (cast `/Game/FirstPerson/Blueprints/BP_FirstPersonCharacter` OtherActor)
  (set `self.canHitPlayer` false))

(event `Set Enemy Type`
  (bind _wc_melee (`self.WC_Melee`))
  (bind _wc_ranged (`self.WC_Ranged`))
  (if (== (`KismetMathLibrary.RandomIntegerInRange` 1 2) 1)
    (set `self.Ranged?` true)
    (`SceneComponent.SetVisibility` _wc_melee false true)
    (`SceneComponent.SetVisibility` _wc_ranged true true)
    (`SceneComponent.K2_AttachToComponent` _wc_ranged (`self.Mesh`) "hand_rSocket_Rifle" "KeepRelative" "KeepRelative" "KeepRelative" true)
    (set `/Game/current_FirstPerson/Blueprints/BP_Weapon_Component_Enemy.ProjectileOffset` (50.0 20.0 0.0) _wc_ranged)
    (else
      (set `self.Ranged?` false)
      (`SceneComponent.SetVisibility` _wc_melee true true)
      (`SceneComponent.SetVisibility` _wc_ranged false true)
      (`SceneComponent.K2_AttachToComponent` _wc_melee (`self.Mesh`) "hand_rSocket_Rifle" "KeepRelative" "KeepRelative" "KeepRelative" true))))

(event `/Game/BP/I_Interact.OnHit`
  (params (Damage :type "Float (double-precision)") (Object :type "/Game/current_FirstPerson/Blueprints/BP_FirstPersonProjectile Object Reference"))
  (bind _returnvalue_location (`KismetMathLibrary.BreakTransform` (`self.GetTransform`)))
  (bind _sounds (`self.Sounds`))
  (`self.RagDollOnHit`)
  (set `self.isAlive` false)
  (if (> (`KismetMathLibrary.RandomIntegerInRange` 0 5) 0)
    (`|SpawnActorFromClass` "/Game/BP/BP_ScorePickup.BP_ScorePickup_C" (`self.GetTransform`) "AdjustIfPossibleButAlwaysSpawn" "MultiplyWithRoot" null null)
    (`NiagaraFunctionLibrary.SpawnSystemAtLocation` "/Game/MegaMagicVFXBundle/VFX/MagicalExplosionsVFX/VFX/BloodExplosion/Systems/N_BloodExplosion.N_BloodExplosion" _returnvalue_location)
    (`GameplayStatics.PlaySoundAtLocation` (`|GetArrayItem` _sounds (`KismetMathLibrary.RandomIntegerInRange` 0 (- (`KismetArrayLibrary.Array_Length` _sounds) 1))) _returnvalue_location (struct) 1.0 1.0 0.0 null null null null)))

(event `self.WeponDamage.OnComponentHit`
  (params (HitComponent :type "PrimitiveComponent Object Reference") (OtherActor :type "Actor Object Reference") (OtherComp :type "PrimitiveComponent Object Reference") (NormalImpulse :type "Vector Structure") (Hit :type "HitResult Structure (by ref)"))
  (bind _asbp_first_person_character (cast `/Game/FirstPerson/Blueprints/BP_FirstPersonCharacter` OtherActor))
  (`/Game/BP/I_Interact.OnHitPlayer` _asbp_first_person_character 0.0 null))

(fn `IsInteractable`
  (returns (isInteractable :type Boolean))
  (return false))

(fn `OnRep_isAlive`
  (bind _returnvalue (`KismetMathLibrary.RandomIntegerInRange` 0 5))
  (if (not (`self.isAlive`))
    (set `self.isDead` true)
    (`self.RagDollOnHit`)
    (if (> _returnvalue 0)
      (for _ (range 1 (+ _returnvalue 1))
        (`|SpawnActorFromClass` "/Game/BP/BP_ScorePickup.BP_ScorePickup_C" (`KismetMathLibrary.Conv_VectorToTransform` (`KismetMathLibrary.RandomPointInBoundingBox_Box` (struct))) "AdjustIfPossibleButAlwaysSpawn" "MultiplyWithRoot" null null)))))

(fn `RagDollOnHit`
  (bind _mesh (`self.Mesh`))
  (`PrimitiveComponent.SetCollisionEnabled` _mesh "QueryAndPhysics")
  (`PrimitiveComponent.SetSimulatePhysics` _mesh true)
  (`SkeletalMeshComponent.SetPhysicsBlendWeight` _mesh 1.0)
  (set `self.isDead` true)
  (`self.SetLifeSpan` 2.0))

(fn `UserConstructionScript`
  (`self.Set Enemy Type`))