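; BP_HealthPickup is a pickup actor that heals the first-person player character when touched.
; Overlapping its sphere casts the other actor to BP_FirstPersonCharacter and calls HealCharacter with the Heal amount.
; It then spawns a Niagara light-blast effect, plays a random sound from its Sound array at its location, and destroys itself.
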(event `self.Sphere.OnComponentBeginOverlap`
  (params (OverlappedComponent :type "PrimitiveComponent Object Reference") (OtherActor :type "Actor Object Reference") (OtherComp :type "PrimitiveComponent Object Reference") (OtherBodyIndex :type Integer) (bFromSweep :type Boolean) (SweepResult :type "HitResult Structure (by ref)"))
  (bind _sound (`self.Sound`))
  (bind _asbp_first_person_character (cast `/Game/FirstPerson/Blueprints/BP_FirstPersonCharacter` OtherActor))
  (`/Game/FirstPerson/Blueprints/BP_FirstPersonCharacter.Heal Character` _asbp_first_person_character (`self.Heal`))
  (`NiagaraFunctionLibrary.SpawnSystemAtLocation` "/Game/MegaMagicVFXBundle/VFX/MagicalExplosionsVFX/VFX/LightBlast/Systems/N_LightBlast.N_LightBlast" (`self.K2_GetActorLocation`))
  (`GameplayStatics.PlaySoundAtLocation` (`|GetArrayItem` _sound (`KismetMathLibrary.RandomIntegerInRange` 0 (- (`KismetArrayLibrary.Array_Length` _sound) 1))) (`self.K2_GetActorLocation`) (struct) 1.0 1.0 0.0 null null null null)
  (`self.K2_DestroyActor`))

(fn `UserConstructionScript`)