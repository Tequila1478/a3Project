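; Maze generator actor that, on BeginPlay, builds room data and spawns a square wall grid of scaled MazeTile_BP actors.
; It fills RoomArray with cell-centre transforms and random door counts, then attempts random start and seeded end assignment, only printing an error on a detected clash.
; The player moves to the first array entry rather than the recorded start room.
; Door counts do not affect the spawned walls.
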(event EventBeginPlay
  (bind _returnvalue (Game|Player|GetPlayerPawn 0))
  (bind _gridsize (Variables|WallGeneration|GetGridSize))
  (bind _scale (Variables|WallGeneration|Getscale))
  (bind _scale_2 (Variables|WallGeneration|Getscale))
  (bind _gridsize_2 (Variables|WallGeneration|GetGridSize))
  (bind _scale_3 (Variables|WallGeneration|Getscale))
  (bind _roomarray (Variables|RoomGeneration|GetRoomArray))
  (bind _roomarray_2 (Variables|RoomGeneration|GetRoomArray))
  (bind _roomarray_3 (Variables|RoomGeneration|GetRoomArray))
  (bind _scale_4 (Variables|WallGeneration|Getscale))
  (bind _gridsize_3 (Variables|WallGeneration|GetGridSize))
  (bind _output (Utilities|Array|Get(acopy) _roomarray_3))
  (bind _returnvalue_2 (/ _scale_2 2))
  (bind _returnvalue_3 (- _gridsize 3))
  (bind _returnvalue_4 (/ _scale_4 100))
  (bind _returnvalue_5 (- _gridsize_3 2))
  (bind _returnvalue_6 (Math|Conversions|ToFloat(Integer) _returnvalue_4))
  (bind _returnvalue_7 (Math|Vector|MakeVector _returnvalue_6 1.0 4.0))
  ;[1 1 1] Creates Array of information to PCG rooms
  (bind _output_get (Variables|RoomGeneration|SetNumOfRooms (* _returnvalue_5 _returnvalue_5)))
  (for _index (range 0 _returnvalue_3)
    (for _index_2 (range 0 _returnvalue_3)
      (Utilities|Array|Add (Variables|RoomGeneration|GetRoomLocationArray) (Math|Transform|MakeTransform (+ (Math|Vector|MakeVector (Math|Conversions|ToFloat(Integer) (* _index_2 _scale)) (Math|Conversions|ToFloat(Integer) (* _index _scale)) 0.0) (+ (.location (Transformation|GetActorTransform)) (Math|Vector|MakeVector _returnvalue_2 _returnvalue_2 0.0)))))))
  (for _index_3 (range 0 (- _output_get 1))
    (Utilities|Array|Add (Variables|RoomGeneration|GetRoomArray) (Utilities|Struct|MakeRoomInfo_Struct (+ _index_3 1) (+ (Math|Random|RandomInteger 2) 2) (Utilities|Array|Get(acopy) (Variables|RoomGeneration|GetRoomLocationArray) _index_3) 0 (Variables|WallGeneration|Getscale))))
  ;;[1 1 1] Once completed assign a random room as the starting room
  (Utilities|Array|SetArrayElem _roomarray_2 (Math|Random|RandomInteger (Variables|RoomGeneration|GetNumOfRooms)) (Utilities|Struct|MakeRoomInfo_Struct (.id (Utilities|Array|Get(acopy) _roomarray_2 (Math|Random|RandomInteger (Variables|RoomGeneration|GetNumOfRooms)))) 0 (.location (Utilities|Array|Get(acopy) _roomarray_2 (Math|Random|RandomInteger (Variables|RoomGeneration|GetNumOfRooms)))) (.numberofdoors (Utilities|Array|Get(acopy) _roomarray_2 (Math|Random|RandomInteger (Variables|RoomGeneration|GetNumOfRooms)))) (.size (Utilities|Array|Get(acopy) _roomarray_2 (Math|Random|RandomInteger (Variables|RoomGeneration|GetNumOfRooms))))))
  (Variables|Default|SetStartingRoomIDNum (.id (Utilities|Array|Get(acopy) _roomarray_2 (Math|Random|RandomInteger (Variables|RoomGeneration|GetNumOfRooms)))))
  (if (== (.type (Utilities|Array|Get(acopy) _roomarray (Class|KismetMathLibrary|RandomIntegerfromStream (Math|Random|MakeRandomStream 0) (Variables|RoomGeneration|GetNumOfRooms)))) 0)
    (Development|PrintString "Error in MazeGenerator_BP, the chosen end point is the start point!!! PLs add logic to stop this")
    (else
      (Utilities|Array|SetArrayElem _roomarray 0 (Utilities|Struct|MakeRoomInfo_Struct (.id (Utilities|Array|Get(acopy) _roomarray (Class|KismetMathLibrary|RandomIntegerfromStream (Math|Random|MakeRandomStream 0) (Variables|RoomGeneration|GetNumOfRooms)))) 1 (.location (Utilities|Array|Get(acopy) _roomarray (Class|KismetMathLibrary|RandomIntegerfromStream (Math|Random|MakeRandomStream 0) (Variables|RoomGeneration|GetNumOfRooms)))) (.numberofdoors (Utilities|Array|Get(acopy) _roomarray (Class|KismetMathLibrary|RandomIntegerfromStream (Math|Random|MakeRandomStream 0) (Variables|RoomGeneration|GetNumOfRooms)))) (.size (Utilities|Array|Get(acopy) _roomarray (Class|KismetMathLibrary|RandomIntegerfromStream (Math|Random|MakeRandomStream 0) (Variables|RoomGeneration|GetNumOfRooms))))))))
  ;;[1 1 1] Move Player to centre of the starting room
  (Transformation|SetActorLocation _returnvalue (Math|Vector|MakeVector (.x (.location (.location _output))) (.y (.location (.location _output))) (.z (Transformation|GetActorLocation _returnvalue))) false false)
  ;[1 1 1] Creates grid gridSize * gridSize with a room length of scale /100
  ;;[1 1 1] Creates Grid
  (for _index_4 (range 0 _gridsize_2)
    (for _index_5 (range 0 _gridsize_2)
      (bind _output_get_2 (Variables|WallGeneration|SetNextPos (+ (Math|Vector|MakeVector (Math|Conversions|ToFloat(Integer) (* _index_5 _scale_3)) (Math|Conversions|ToFloat(Integer) (* _index_4 _scale_3)) 0.0) (Transformation|GetActorLocation))))
      (Game|SpawnActorfromClass "/Game/BP/MazeTile_BP.MazeTile_BP_C" (Math|Transform|MakeTransform _output_get_2 "0, 0, 0" _returnvalue_7) "Undefined" "MultiplyWithRoot" 0 0)
      (Game|SpawnActorfromClass "/Game/BP/MazeTile_BP.MazeTile_BP_C" (Math|Transform|MakeTransform _output_get_2 "0.000000,90.000000,0.000000" _returnvalue_7) "Undefined" "MultiplyWithRoot" 0 0))))

(event Collision|EventActorBeginOverlap
  (params (OtherActor :type Actor%20Object%20Reference)))

(event EventTick
  (params (DeltaSeconds :type Float%20%28single-precision%29)))

(fn ConstructionScript)