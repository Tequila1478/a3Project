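; Score pickup actor that awards a random point value to the first-person player character on overlap.
; On BeginPlay it rolls an integer Worth and scales its root uniformly with that value, clamped to a range, so bigger pickups are worth more.
; Sphere overlap adds the points to the character, spawns a Niagara explosion, plays a random sound from an array and destroys the actor.
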(event `self.ReceiveBeginPlay`
  (bind _output_get (set `self.Worth` (`KismetMathLibrary.RandomIntegerInRange` 1 10)))
  (bind _returnvalue (`KismetMathLibrary.FClamp` (* (/ (`KismetMathLibrary.Conv_IntToDouble` _output_get) 10.0) 0.5) 0.1 0.5))
  (`SceneComponent.SetWorldScale3D` (`self.DefaultSceneRoot`) (`KismetMathLibrary.MakeVector` _returnvalue _returnvalue _returnvalue)))

(event `self.Sphere.OnComponentBeginOverlap`
  (params (OverlappedComponent :type "PrimitiveComponent Object Reference") (OtherActor :type "Actor Object Reference") (OtherComp :type "PrimitiveComponent Object Reference") (OtherBodyIndex :type Integer) (bFromSweep :type Boolean) (SweepResult :type "HitResult Structure (by ref)"))
  (bind _sounds (`self.Sounds`))
  (bind _asbp_first_person_character (cast `/Game/FirstPerson/Blueprints/BP_FirstPersonCharacter` OtherActor))
  (`/Game/FirstPerson/Blueprints/BP_FirstPersonCharacter.Add Points` _asbp_first_person_character (`KismetMathLibrary.Conv_IntToDouble` (`self.Worth`)))
  (`NiagaraFunctionLibrary.SpawnSystemAtLocation` "/Game/MegaMagicVFXBundle/VFX/MagicalExplosionsVFX/VFX/MagicalExplosion/Systems/N_MagicalExplosion.N_MagicalExplosion" (`self.K2_GetActorLocation`))
  (`GameplayStatics.PlaySoundAtLocation` (`|GetArrayItem` _sounds (`KismetMathLibrary.RandomIntegerInRange` 0 (- (`KismetArrayLibrary.Array_Length` _sounds) 1))) (`self.K2_GetActorLocation`) (struct) 1.0 1.0 0.0 null null null null)
  (`self.K2_DestroyActor`))

(fn `UserConstructionScript`)